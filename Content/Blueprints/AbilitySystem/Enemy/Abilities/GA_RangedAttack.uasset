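; Enemy ranged attack Gameplay Ability, so far without projectile or damage logic.
; On activation it turns the avatar toward its combat target through the CombatInterface and plays a random tagged attack montage.
; The montage's tag serves as the awaited gameplay event, which currently only draws a debug sphere at the matching combat socket.
; The ability ends when the montage completes or is interrupted or cancelled; the local GetRandomAttackMontage helper is not called.
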(event Ability|EventActivateAbility
  (bind _output_get (Variables|Default|SetAvatarActor (Ability|GetAvatarActorfromActorInfo)))
  ;[0.6529 0.5194 0.2053 0.5] Facing to Target
  (bind _returnvalue (Class|EnemyInterface|GetCombatTarget(Message) _output_get))
  (bind _ascombat_interface (Utilities|Casting|CastToCombatInterface (Variables|Default|GetAvatarActor)))
  (Class|CombatInterface|SetFacingTarget _ascombat_interface (Transformation|GetActorLocation _returnvalue))
  ;[0.09593 0.1737 0.7661 0.5] Play Montage
  (bind _returnvalue_2 (Class|CombatInterface|GetAttackMontages(Message) (Variables|Default|GetAvatarActor)))
  (Variables|Default|SetAttackMontage (Class|AuraDamageGameplayAbility|GetRandomTaggedMontage _returnvalue_2))
  (|PlayMontageandWaitProxy "None" (.Montage (Utilities|Struct|BreakTaggedMontage (Variables|Default|GetAttackMontage))) 1.0 "None" false 1.0 0.0 false
    (:then
      (Ability|Tasks|WaitGameplayEvent (.MontageTag (Utilities|Struct|BreakTaggedMontage (Variables|Default|GetAttackMontage))) 0
        (:EventReceived
          (bind _returnvalue_3 (Class|CombatInterface|GetCombatSocketLocation(Message) (Variables|Default|GetAvatarActor) (.MontageTag (Utilities|Struct|BreakTaggedMontage (Variables|Default|GetAttackMontage)))))
          (Rendering|Debug|DrawDebugSphere _returnvalue_3 5.0 12 "(R=1.000000,G=1.000000,B=1.000000,A=1.000000)" 3.0))))
    (:OnCompleted
      (Ability|EndAbility :!label _label))
    (:OnInterrupted
      (goto _label))
    (:OnCancelled
      (goto _label))))

(fn GetRandomAttackMontage
  (bind _returnvalue (Class|CombatInterface|GetAttackMontages(Message) (Variables|Default|GetAvatarActor)))
  (if (> (Utilities|Array|Length _returnvalue) 0)
    (return (Utilities|Array|Get(acopy) _returnvalue (Math|Random|RandomIntegerinRange 0 (- (Utilities|Array|Length _returnvalue) 1))))
    (else
      (Ability|EndAbility))))