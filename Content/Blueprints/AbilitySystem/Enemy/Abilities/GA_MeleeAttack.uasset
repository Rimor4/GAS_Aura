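; Gameplay ability for an enemy melee attack that turns the avatar toward its combat target and plays a random attack montage.
; The montage and its event tag come from the avatar's attack montage list.
; When that tagged gameplay event arrives, it finds live players within the enemy's physical attack radius around the matching combat socket and damages those on another team.
; The ability ends after the hit or when the montage finishes or is interrupted.
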(event Ability|EventActivateAbility
  (bind _output_get (Variables|Default|SetAvatarActor (Ability|GetAvatarActorfromActorInfo)))
  ;[0.6529 0.5194 0.2053 0.5] Facing to Target
  (bind _returnvalue (Class|EnemyInterface|GetCombatTarget(Message) _output_get))
  (bind _ascombat_interface (Utilities|Casting|CastToCombatInterface (Variables|Default|GetAvatarActor)))
  (Class|CombatInterface|SetFacingTarget _ascombat_interface (Transformation|GetActorLocation _returnvalue))
  ;[0.09593 0.1737 0.7661 0.5] Play Montage
  (bind _attackmontage (CallFunction|GetRandomAttackMontage))
  (Variables|Default|SetAttackMontage _attackmontage)
  (|PlayMontageandWaitProxy "None" (.Montage (Utilities|Struct|BreakTaggedMontage (Variables|Default|GetAttackMontage))) 1.0 "None" false 1.0 0.0 false
    (:then
      (Ability|Tasks|WaitGameplayEvent (.MontageTag (Utilities|Struct|BreakTaggedMontage (Variables|Default|GetAttackMontage))) 0
        (:EventReceived
          ;[0.8363 0.1388 0.1669 0.5] Cause Damage to Targets
          (bind _asaura_enemy (Utilities|Casting|CastToAuraEnemy (Variables|Default|GetAvatarActor))
            (:then
              (bind _returnvalue_2 (Class|CombatInterface|GetCombatSocketLocation(Message) (Variables|Default|GetAvatarActor) (.MontageTag (Utilities|Struct|BreakTaggedMontage (Variables|Default|GetAttackMontage)))))
              (bind _outactors (Class|AuraAbilitySystemLibrary|GetLivePlayersWithinRadius (Variables|Default|GetAvatarActor) (Utilities|Array|MakeArray (Variables|Default|GetAvatarActor)) _returnvalue_2 (Variables|/Script/Aura.AuraEnemy|GetPhysicalAttackRadius _asaura_enemy)))
              (for _array_element _outactors
                (if (not (Class|AuraAbilitySystemLibrary|IsSameTeam (Variables|Default|GetAvatarActor) _array_element))
                  (Class|AuraDamageGameplayAbility|CauseDamage _array_element)))
              (Ability|EndAbility))
            (:CastFailed
              (Ability|EndAbility))))))
    (:OnCompleted
      (Ability|EndAbility :!label _label))
    (:OnInterrupted
      (goto _label))
    (:OnCancelled
      (goto _label))))

(fn GetRandomAttackMontage
  (bind _returnvalue (Class|CombatInterface|GetAttackMontages(Message) (Variables|Default|GetAvatarActor)))
  (if (> (Utilities|Array|Length _returnvalue) 0)
    (return (Utilities|Array|Get(acopy) _returnvalue (Math|Random|RandomIntegerinRange 0 (- (Utilities|Array|Length _returnvalue) 1))))
    (else
      (Ability|EndAbility))))